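; BP_Battery is a battery pickup that adds one to the first-person character's ExtraBatteries count.
; BeginPlay caches player 0's character as BP_FirstPersonCharacter.
; Any overlap on the Capsule, with no check on the overlapping actor, plays a click sound, increments that count, destroys the pickup and prints the total on screen.
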(event `self.ReceiveBeginPlay`
  (bind _asbp_first_person_character (cast `/Game/FPS_TARGET_PRACTICE/Blueprints/BP_FirstPersonCharacter` (`GameplayStatics.GetPlayerCharacter` 0)))
  (set `self.PlayereREF` _asbp_first_person_character))

(event `self.Capsule.OnComponentBeginOverlap`
  (params (OverlappedComponent :type "PrimitiveComponent Object Reference") (OtherActor :type "Actor Object Reference") (OtherComp :type "PrimitiveComponent Object Reference") (OtherBodyIndex :type Integer) (bFromSweep :type Boolean) (SweepResult :type "HitResult Structure (by ref)"))
  (`GameplayStatics.PlaySoundAtLocation` "/Engine/VREditor/Sounds/UI/Click_on_Button.Click_on_Button" (`self.K2_GetActorLocation`) (struct) 1.0 1.0 0.0 null null null null)
  (set `/Game/FPS_TARGET_PRACTICE/Blueprints/BP_FirstPersonCharacter.ExtraBatteries` (+ (`/Game/FPS_TARGET_PRACTICE/Blueprints/BP_FirstPersonCharacter.ExtraBatteries` (`self.PlayereREF`)) 1.0) (`self.PlayereREF`))
  (`|ExecutionSequence`
    (:`then_0`
      (`self.K2_DestroyActor`))
    (:`then_1`
      (`KismetSystemLibrary.PrintString` (`KismetStringLibrary.Conv_DoubleToString` (`/Game/FPS_TARGET_PRACTICE/Blueprints/BP_FirstPersonCharacter.ExtraBatteries` (`self.PlayereREF`))) true true (struct :`G` 0.66 :`B` 1.0 :`A` 1.0) 4.0))
    (:`then_2`
      (`KismetSystemLibrary.PrintString` "Batteries Remaining" true true (struct :`G` 0.66 :`B` 1.0 :`A` 1.0) 4.0))))

(fn `UserConstructionScript`)