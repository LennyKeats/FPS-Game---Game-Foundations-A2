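; BP_Key_Red is a red key pickup that stays hidden and non-collidable until no actors tagged "TARGET" remain.
; Tick recounts tagged actors, using an array Add index as the count, prints it, and toggles visibility and collision.
; A DoOnce plays the appearance particle and sound.
; When the cached first-person player overlaps the capsule, the key sets HasKeyRed, plays a collect sound and destroys itself.
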(event `self.Capsule Collision Box.OnComponentBeginOverlap`
  (params (OverlappedComponent :type "PrimitiveComponent Object Reference") (OtherActor :type "Actor Object Reference") (OtherComp :type "PrimitiveComponent Object Reference") (OtherBodyIndex :type Integer) (bFromSweep :type Boolean) (SweepResult :type "HitResult Structure (by ref)"))
  (bind _playerreference (`self.PlayerReference`))
  ; Key Pickup and Destroy
  (if (== OtherActor _playerreference)
    (set `/Game/FPS_TARGET_PRACTICE/Blueprints/BP_FirstPersonCharacter.HasKeyRed` true _playerreference)
    (`GameplayStatics.PlaySoundAtLocation` "/Game/FPS_TARGET_PRACTICE/SFX/MP3_Key_Collect.MP3_Key_Collect" (`self.K2_GetActorLocation`) (struct) 1.0 1.0 0.0 null null null null)
    (`self.K2_DestroyActor`)))

(event `self.ReceiveBeginPlay`
  ; Setup Variable
  (bind _asbp_first_person_character (cast `/Game/FPS_TARGET_PRACTICE/Blueprints/BP_FirstPersonCharacter` (`GameplayStatics.GetPlayerCharacter` 0)))
  (set `self.PlayerReference` _asbp_first_person_character))

(event `self.ReceiveTick`
  (params (DeltaSeconds :type "Float (single-precision)"))
  (bind _returnvalue (`SceneComponent.K2_GetComponentLocation` (`self.DefaultSceneRoot`)))
  ;[0.15 0.1214 0.005804 0.5] Key-Visibility
  (bind _outactors (`GameplayStatics.GetAllActorsWithTag` "TARGET"))
  (bind _returnvalue_2 (`KismetArrayLibrary.Array_Add` _outactors))
  (`|ExecutionSequence`
    (:`then_0`
      (bind _returnvalue_3 (<= _returnvalue_2 0))
      (`SceneComponent.SetVisibility` (`self.DefaultSceneRoot`) _returnvalue_3 true)
      (`self.SetActorEnableCollision` _returnvalue_3)
      ; Key Spawn Effect
      (if _returnvalue_3
        (`/Engine/EditorBlueprintResources/StandardMacros.DoOnce` false
          (:`Completed`
            (`GameplayStatics.SpawnEmitterAtLocation` "/Engine/Tutorial/SubEditors/TutorialAssets/TutorialParticleSystem.TutorialParticleSystem" _returnvalue)
            (`GameplayStatics.PlaySoundAtLocation` "/Game/FPS_TARGET_PRACTICE/SFX/MP3_Key_Appear.MP3_Key_Appear" _returnvalue (struct) 1.0 1.0 0.0 null null null null)))))
    (:`then_1`
      (`KismetSystemLibrary.PrintString` (`KismetStringLibrary.Conv_IntToString` _returnvalue_2) true true (struct :`R` 1.0 :`B` 0.006009 :`A` 1.0)))))

(fn `UserConstructionScript`)