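; BP_Camera is a rotating stealth security camera that restarts play in Lvl_Stealth when it spots the player.
; BeginPlay caches the first-person character and starts a self-calling MoveCamera loop that FlipFlops the camera mesh between two rotations with a pause.
; Every Tick, a debug-drawn Pawn line trace runs forward from the LineTrace component.
; Hitting the player disables input and opens the level after a delay.
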(event `DetectPlayer`
  (bind _linetrace (`self.LineTrace`))
  (bind _returnvalue (`SceneComponent.K2_GetComponentLocation` _linetrace))
  (bind _outhit (`KismetSystemLibrary.LineTraceSingleForObjects` :`Start` _returnvalue :`End` (+ _returnvalue (* (`KismetMathLibrary.GetForwardVector` (`SceneComponent.K2_GetComponentRotation` _linetrace)) (`self.DetectionRange`))) :`ObjectTypes` (`|MakeArray` "ObjectTypeQuery3" :!type "EObjectTypeQuery Enum") :`DrawDebugType` "ForOneFrame"))
  (if (== (`.HitActor` (`GameplayStatics.BreakHitResult` _outhit)) (`self.Player Reference`))
    (`KismetSystemLibrary.PrintString` "raaa")
    (`self.DisableInput` (`self.Player Reference`) (`GameplayStatics.GetPlayerController` 0))
    (`KismetSystemLibrary.Delay` 2.0)
    (`GameplayStatics.OpenLevel` "Lvl_Stealth")))

(event `self.ReceiveTick`
  (params (DeltaSeconds :type "Float (single-precision)"))
  (`self.DetectPlayer`))

(event `MoveCamera`
  ; Rotate Camera
  (`/Engine/EditorBlueprintResources/StandardMacros.FlipFlop`
    (:`A`
      (set `self.CurrentRotation` (`self.EndRotation`)))
    (:`B`
      (set `self.CurrentRotation` (`self.StartRotation`))))
  (`KismetSystemLibrary.MoveComponentTo` (`self.SM_Camera`) (0.0 0.0 0.0) (`self.CurrentRotation`) false false (`self.RotationSpeed`))
  (`KismetSystemLibrary.Delay` (`self.Delay`))
  (`self.MoveCamera`))

(event `self.ReceiveBeginPlay`
  ; Rotate Camera
  (`|ExecutionSequence`
    (:`then_0`
      (`self.MoveCamera`))
    (:`then_1`
      (bind _asbp_first_person_character (cast `/Game/FPS_TARGET_PRACTICE/Blueprints/BP_FirstPersonCharacter` (`GameplayStatics.GetPlayerCharacter` 0)))
      (set `self.Player Reference` _asbp_first_person_character))))

(event `EnhancedInput|/Game/FPS_TARGET_PRACTICE/Inputs/IA_EMP`
  (params (ActionValue :type Boolean) (ElapsedSeconds :type "Float (double-precision)") (TriggeredSeconds :type "Float (double-precision)") (InputAction :type "InputAction Object Reference" :default "/Game/FPS_TARGET_PRACTICE/Inputs/IA_EMP.IA_EMP")))

(fn `UserConstructionScript`)