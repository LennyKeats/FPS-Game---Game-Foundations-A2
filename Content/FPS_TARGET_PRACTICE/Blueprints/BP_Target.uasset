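; BP_Target is a moving shooting-range target that takes hits and breaks when its hit points run out.
; Each Hit event removes a hit point and spawns a hit effect, or a break effect before destroying the actor on the final hit.
; Tick moves it along its normalized Direction by Speed without scaling by delta time, while a looping timer reverses Direction every MovementDuration to make it patrol back and forth.
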(event `self.ReceiveHit`
  (params (MyComp :type "PrimitiveComponent Object Reference") (Other :type "Actor Object Reference") (OtherComp :type "PrimitiveComponent Object Reference") (bSelfMoved :type Boolean) (HitLocation :type "Vector Structure") (HitNormal :type "Vector Structure") (NormalImpulse :type "Vector Structure") (Hit :type "HitResult Structure (by ref)"))
  ; Target DMG on hit -> despawn
  (set `self.HitPoints` (- (`self.HitPoints`) 1))
  (if (<= (`self.HitPoints`) 0)
    (`NiagaraFunctionLibrary.SpawnSystemAtLocation` "/Game/FPS_TARGET_PRACTICE/FX/PE_Target_Break.PE_Target_Break" HitLocation)
    (`self.K2_DestroyActor`)
    (else
      (`NiagaraFunctionLibrary.SpawnSystemAtLocation` "/Game/FPS_TARGET_PRACTICE/FX/PE_Target_Hit.PE_Target_Hit" HitLocation (struct) (5.0 5.0 5.0)))))

(event `self.ReceiveBeginPlay`
  ; Flip Direction Each 3 Seconds
  (`KismetSystemLibrary.K2_SetTimerDelegate` (delegate `Flip Direction`) (`self.MovementDuration`) true))

(event `Flip Direction`
  ; Flip Direction Each 3 Seconds
  (set `self.Direction` (* (`self.Direction`) -1.0)))

(event `self.ReceiveTick`
  (params (DeltaSeconds :type "Float (single-precision)"))
  ; Determines target MOVEMENT
  (`self.K2_AddActorWorldOffset` (* (`KismetMathLibrary.Normal` (`self.Direction`)) (`self.Speed`))))

(fn `UserConstructionScript`)