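; BP_Door is a key-locked door that swings open when the player enters its trigger zone holding a key.
; BeginPlay caches the first-person character and creates a dynamic material instance for the door light.
; On overlap, the light brightens and turns green or red based on HasKey, with green playing a timeline that rotates the door mesh 90 degrees.
; Leaving the zone dims the light to yellow and reverses the timeline to close the door.
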(event `self.Door_TriggerZone.OnComponentEndOverlap`
  (params (OverlappedComponent :type "PrimitiveComponent Object Reference") (OtherActor :type "Actor Object Reference") (OtherComp :type "PrimitiveComponent Object Reference") (OtherBodyIndex :type Integer))
  ; Reset Door
  (if (== (`self.PlayerReference`) OtherActor)
    (`MaterialInstanceDynamic.SetScalarParameterValue` (`self.Door Light`) "Emission" 100.0)
    (`MaterialInstanceDynamic.SetVectorParameterValue` (`self.Door Light`) "Colour" (struct :`R` 0.9375 :`G` 0.815026 :`B` 0.13688 :`A` 1.0))
    ; Door Open/Close
    (bind (_direction _alpha) (`Timeline|Timeline_DoorOpenClose` :!via `Reverse` :!label _label)
      (:`Update`
        (set `self.DoorOpening` true)
        (`SceneComponent.K2_SetRelativeRotation` (`self.SM_Door`) (`KismetMathLibrary.RLerp` (struct) (struct :`Yaw` 90.0) _alpha) false false))
      (:`Finished`
        (set `self.DoorOpening` false)))))

(event `self.Door_TriggerZone.OnComponentBeginOverlap`
  (params (OverlappedComponent :type "PrimitiveComponent Object Reference") (OtherActor :type "Actor Object Reference") (OtherComp :type "PrimitiveComponent Object Reference") (OtherBodyIndex :type Integer) (bFromSweep :type Boolean) (SweepResult :type "HitResult Structure (by ref)"))
  ; Change Door Colour
  (if (== (`self.PlayerReference`) OtherActor)
    (`MaterialInstanceDynamic.SetScalarParameterValue` (`self.Door Light`) "Emission" 200.0)
    (if (`/Game/FPS_TARGET_PRACTICE/Blueprints/BP_FirstPersonCharacter.HasKey` (`self.PlayerReference`))
      (`MaterialInstanceDynamic.SetVectorParameterValue` (`self.Door Light`) "Colour" (struct :`G` 1.0 :`A` 1.0))
      (goto _label)
      (else
        (`MaterialInstanceDynamic.SetVectorParameterValue` (`self.Door Light`) "Colour" (struct :`R` 1.0 :`A` 1.0))))))

(event `self.ReceiveBeginPlay`
  ; Change Door Colour
  (`|ExecutionSequence`
    (:`then_0`
      (bind _asbp_first_person_character (cast `/Game/FPS_TARGET_PRACTICE/Blueprints/BP_FirstPersonCharacter` (`GameplayStatics.GetPlayerCharacter` 0)))
      (set `self.PlayerReference` _asbp_first_person_character))
    (:`then_1`
      (bind _returnvalue (`KismetMaterialLibrary.CreateDynamicMaterialInstance` "/Game/FPS_TARGET_PRACTICE/Materials/MI_DoorLight.MI_DoorLight"))
      (bind _output_get (set `self.Door Light` _returnvalue))
      (`PrimitiveComponent.SetMaterial` (`self.SM_DoorLight`) 0 _output_get))))

(fn `UserConstructionScript`)